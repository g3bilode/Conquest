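; Barracks Blueprint for the Conquest game that exposes a fixed set of six unit spawn points.
; Each slot is a child actor component whose spawned actor is cast to SpawnPoint by a helper function.
; On BeginPlay the results fill the UnitSlots array in component order; the file holds no spawning logic itself.
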(event EventBeginPlay
  ;[1 1 1] Init UnitSlot array
  (Variables|Default|SetUnitSlots (Utilities|Array|MakeArray (CallFunction|GetSpawnPointfromComponent (Variables|Default|GetUnitSpawnPoint_0)) (CallFunction|GetSpawnPointfromComponent (Variables|Default|GetUnitSpawnPoint_1)) (CallFunction|GetSpawnPointfromComponent (Variables|Default|GetUnitSpawnPoint_2)) (CallFunction|GetSpawnPointfromComponent (Variables|Default|GetUnitSpawnPoint_3)) (CallFunction|GetSpawnPointfromComponent (Variables|Default|GetUnitSpawnPoint_4)) (CallFunction|GetSpawnPointfromComponent (Variables|Default|GetUnitSpawnPoint_5)))))

(fn ConstructionScript)

(fn GetSpawnPointfromComponent
  (params (ChildActorComponent :type Child%20Actor%20Component%20Object%20Reference))
  (return (.AsSpawn%20Point (Utilities|Casting|CastToSpawnPoint (Variables|/Script/Engine.ChildActorComponent|GetChildActor ChildActorComponent)))))