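; Capture point for Conquest that reports unit contact per team and shows which team occupies it.
; Two trigger volumes, each bound to a target team, filter overlaps to components named "HitSphere" on a ConquestUnit of that team.
; Matches call OnTriggerOverlapWithUnit with the team index; capture logic is not in this graph.
; DisplayCapture swaps the plane's material according to OccupierTeamIndex, with a default for other values.
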(event OnComponentBeginOverlap(Trigger_1)
  (params (OverlappedComponent :type Primitive%20Component%20Object%20Reference) (OtherActor :type Actor%20Object%20Reference) (OtherComp :type Primitive%20Component%20Object%20Reference) (OtherBodyIndex :type Integer) (bFromSweep :type Boolean) (SweepResult :type Hit%20Result%20Structure%20%28by%20ref%29))
  (CallFunction|CheckTriggerCollision OtherActor OtherComp (Variables|Default|GetTriggerTarget_1)))

(event OnComponentBeginOverlap(Trigger_0)
  (params (OverlappedComponent :type Primitive%20Component%20Object%20Reference) (OtherActor :type Actor%20Object%20Reference) (OtherComp :type Primitive%20Component%20Object%20Reference) (OtherBodyIndex :type Integer) (bFromSweep :type Boolean) (SweepResult :type Hit%20Result%20Structure%20%28by%20ref%29))
  (CallFunction|CheckTriggerCollision OtherActor OtherComp (Variables|Default|GetTriggerTarget_0)))

(event Custom|CallTriggerEvent
  (params (OtherActor :type Actor%20Object%20Reference) (TriggerTarget :type Integer))
  (bind _asconquest_unit (Utilities|Casting|CastToConquestUnit OtherActor))
  (if (== (Variables|/Script/Conquest.ConquestUnit|GetTeamIndex _asconquest_unit) TriggerTarget)
    (Class|CapturePoint|OnTriggerOverlapwithUnit (Variables|/Script/Conquest.ConquestUnit|GetTeamIndex _asconquest_unit))))

(event EventDisplayCapture
  (switch int (Variables|Default|GetOccupierTeamIndex)
    (:Default
      (Variables|Default|SetCurrentMaterial "/Game/Conquest/Blueprints/CapturePoints/CaptureMaterial_Default.CaptureMaterial_Default"))
    (:0
      (Variables|Default|SetCurrentMaterial "/Game/Conquest/Blueprints/CapturePoints/CaptureMaterial_0.CaptureMaterial_0"))
    (:1
      (Variables|Default|SetCurrentMaterial "/Game/Conquest/Blueprints/CapturePoints/CaptureMaterial_1.CaptureMaterial_1")))
  (Rendering|Material|SetMaterial (Variables|Default|GetPlane) 0 (Variables|Default|GetCurrentMaterial)))

(fn ConstructionScript)

(fn CheckTriggerCollision
  (params (OtherActor :type Actor%20Object%20Reference) (OtherComp :type Primitive%20Component%20Object%20Reference) (TriggerTarget :type Integer))
  (if (Utilities|Enum|Equal(Enum) "HitSphere" (Utilities|GetObjectName OtherComp))
    (CallFunction|CallTriggerEvent OtherActor TriggerTarget)))