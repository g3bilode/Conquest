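; ConquestGameMode is the game mode for Conquest, tracking connected players, assigning teams and handing out gold income.
; PostLogin adds each ConquestPlayerState to CurrentPlayers and uses the resulting array index to pick its team name from TeamDefinitions.
; A looping timer started on BeginPlay adds base gold gain, scaled by each player's multiplier, to that player's Gold.
; The ChoosePlayerStart override is unfinished, only casting the controller without selecting a start.
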(event Custom|UpdateResources
  ;[1 1 1] Update Resources
  (for _array_element (Variables|Default|GetCurrentPlayers)
    (bind _asconquest_player_state (Utilities|Casting|CastToConquestPlayerState _array_element))
    (Utilities|IsValid _asconquest_player_state
      (:Is%20Valid
        (Variables|/Script/Conquest.ConquestPlayerState|SetGold _asconquest_player_state (+ (* (Variables|Resources|GetGoldGainBase) (Variables|/Script/Conquest.ConquestPlayerState|GetGoldGainMultiplayer _asconquest_player_state)) (Variables|/Script/Conquest.ConquestPlayerState|GetGold _asconquest_player_state))))
      (:Is%20Not%20Valid
        (Development|PrintString "==== UPDATE RESOURCES FAILED CAST ====")))))

(event EventBeginPlay
  (Utilities|Time|SetTimerbyEvent (delegate Custom|UpdateResources) (Variables|Resources|GetUpdateResourceTimer) true))

(event EventPostLogin
  (params (NewPlayer :type Player%20Controller%20Object%20Reference))
  ;[1 1 1] Gather Connected Players
  (bind _asconquest_player_state (Utilities|Casting|CastToConquestPlayerState (Variables|/Script/Engine.Controller|GetPlayerState NewPlayer))
    (:then
      (bind _returnvalue (Utilities|Array|Add (Variables|Default|GetCurrentPlayers) _asconquest_player_state))
      (Variables|/Script/Conquest.ConquestPlayerState|SetTeamName _asconquest_player_state (.Name (Utilities|Struct|BreakTeamDefinition (Utilities|Array|Get(acopy) (Variables|Default|GetTeamDefinitions) _returnvalue)))))
    (:CastFailed
      (Development|PrintString "==== JOINED PLAYER FAILED CAST ===="))))

(fn ConstructionScript)

(fn ChoosePlayerStart
  (params (Player :type Controller%20Object%20Reference))
  (bind _asconquest_player_controller (Utilities|Casting|CastToConquestPlayerController Player)))