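; ConquestPlayerState is the player state Blueprint for the Conquest mode, with a team definition and a Gold RepNotify whose handler is empty.
; BeginPlay and AttemptSpawnUnit are empty events, and the graph's remaining logic is disconnected.
; That unused logic would store the location of the UnitSpawnPoint matching the team name and forward spawn requests to the game mode with the player controller, printing errors if either is invalid.
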(event Custom|AttemptSpawnUnit)

(event EventBeginPlay)

(fn ConstructionScript)

(fn OnRepGold)