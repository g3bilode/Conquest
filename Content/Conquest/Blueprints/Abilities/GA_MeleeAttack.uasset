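; GA_MeleeAttack is a gameplay ability that performs a unit's melee attack and damages its current target.
; On activation it has the owner's AttackComponent play the attack animation, then waits once for a MeleeA gameplay event.
; When that event arrives it applies GE_Damage to the component's current target and ends the ability.
; Stored async tasks are ended when the ability ends.
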(event Custom|Event%20ApplyEffect
  (GameplayEffects|ApplyGameplayEffectToTarget (Ability|TargetData|AbilityTargetDatafromActor (Class|AttackComponent|GetCurrentTarget (Variables|Default|GetAttackComponent))) "/Game/Conquest/Blueprints/Abilities/GE_Damage.GE_Damage_C" 1 1)
  (Ability|EndAbility))

(event Ability|EventActivateAbility
  (bind _output_get (Variables|Default|SetAttackComponent (Actor|GetComponentbyClass (.OwnerActor (Utilities|Struct|BreakGameplayAbilityActorInfo (Ability|GetActorInfo))) "/Script/Conquest.AttackComponent")))
  (Class|AttackComponent|PlayAttackAnim _output_get)
  ;[1 1 1] Wait OnHit
  (bind _asynctaskproxy (Ability|Tasks|WaitGameplayEvent (Variables|Default|GetMelee_A) 0 true)
    (:then
      (Utilities|Array|Add (Variables|Default|GetAsyncTasks) _asynctaskproxy))
    (:EventReceived
      (CallFunction|EventApplyEffect))))

(event Ability|EventOnEndAbility
  (params (bWasCancelled :type Boolean))
  (for _array_element (Variables|Default|GetAsyncTasks)
    (Utilities|IsValid _array_element
      (:Is%20Valid
        (GameplayTasks|EndTask _array_element)))))