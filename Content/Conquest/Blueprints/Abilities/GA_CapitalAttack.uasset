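; GA_CapitalAttack is a gameplay ability that performs a capital's attack on the owner's current target.
; On activation it gets the owner's AttackComponent and uses its current target for both the visual and the damage.
; It draws a brief debug line as a placeholder attack animation, applies the GE_Damage effect to that target, then ends the ability.
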(event Ability|EventActivateAbility
  (bind _returnvalue (Ability|GetActorInfo))
  (bind _owneractor (Utilities|Struct|BreakGameplayAbilityActorInfo _returnvalue))
  (bind _output_get (Variables|Default|SetAttackComponent (Actor|GetComponentbyClass _owneractor "/Script/Conquest.AttackComponent")))
  ;[0.402 0.0999 0.5029] Temp Capital Attack "anim"
  (Rendering|Debug|DrawDebugLine (Transformation|GetActorLocation (Class|AttackComponent|GetCurrentTarget _output_get)) (Transformation|GetActorLocation _owneractor) "(R=0.400000,G=0.100000,B=0.500000,A=1.000000)" 1.0 0.0)
  ;[1 1 1] Apply Damage
  (GameplayEffects|ApplyGameplayEffectToTarget (Ability|TargetData|AbilityTargetDatafromActor (Class|AttackComponent|GetCurrentTarget _output_get)) "/Game/Conquest/Blueprints/Abilities/GE_Damage.GE_Damage_C" 1 1)
  (Class|GameplayAbility|EndAbilityState "None"))