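; Blueprint function library for the Conquest game that provides typed shortcuts to its core gameplay framework objects.
; Each getter fetches the game mode, game state or player controller and casts it to its Conquest class.
; The controller getter always uses player index 0 and is the only one that prints a message when the cast fails.
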(fn GetConquestGameMode
  (return (.AsConquest%20Game%20Mode (Utilities|Casting|CastToConquestGameMode (Game|GetGameMode)))))

(fn GetConquestPlayerController
  (bind _asconquest_player_controller (Utilities|Casting|CastToConquestPlayerController (Game|GetPlayerController 0))
    (:then
      (return _asconquest_player_controller))
    (:CastFailed
      (Development|PrintString 0 "FAILED CONQUESTPLAYERCONTROLLER CAST")
      (return 0))))

(fn GetConquestGameState
  (return (.AsConquest%20Game%20State (Utilities|Casting|CastToConquestGameState (Game|GetGameState)))))