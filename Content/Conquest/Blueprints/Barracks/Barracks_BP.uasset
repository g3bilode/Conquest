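; Barracks actor for the Conquest game that holds six unit slots, each placed as a Child Actor Component.
; On BeginPlay it casts each component's child actor to UnitSlot through a helper function and caches the results in the UnitSlots array.
; The construction script is empty, and the file contains no further logic for using the slots.
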(event EventBeginPlay
  ;[1 1 1] Init UnitSlot array
  (Variables|Default|SetUnitSlots (Utilities|Array|MakeArray (CallFunction|GetUnitSlotfromComponent (Variables|Default|GetUnitSlot_0)) (CallFunction|GetUnitSlotfromComponent (Variables|Default|GetUnitSlot_1)) (CallFunction|GetUnitSlotfromComponent (Variables|Default|GetUnitSlot_2)) (CallFunction|GetUnitSlotfromComponent (Variables|Default|GetUnitSlot_3)) (CallFunction|GetUnitSlotfromComponent (Variables|Default|GetUnitSlot_4)) (CallFunction|GetUnitSlotfromComponent (Variables|Default|GetUnitSlot_5)))))

(fn ConstructionScript)

(fn GetUnitSlotfromComponent
  (params (ChildActorComponent :type Child%20Actor%20Component%20Object%20Reference))
  (return (.AsUnit%20Slot (Utilities|Casting|CastToUnitSlot (Variables|/Script/Engine.ChildActorComponent|GetChildActor ChildActorComponent)))))